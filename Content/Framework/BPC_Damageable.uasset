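; BPC_Damageable is a component that gives its owning actor health and handles damage and death.
; It sets current life from an initial value on BeginPlay, and GetDamage subtracts damage while the damageable flag is on.
; A non-lethal hit fires OnGetDamage with remaining HP and the damager, then prints the HP.
; At zero it clamps life, fires OnDeath and optionally destroys the owner.
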(event EventBeginPlay
  (Variables|Default|SetCurrentLife (Variables|Default|GetInitialLife)))

(event EventTick
  (params (DeltaSeconds :type Float%20%28single-precision%29)))

(fn GetDamage
  (params (Damage :type Float%20%28double-precision%29) (Damager :type Actor%20Object%20Reference))
  (if (Variables|Default|GetCanBeDamagable)
    (bind _output_get (Variables|Default|SetCurrentLife (- (Variables|Default|GetCurrentLife) Damage)))
    (if (<= _output_get 0.0)
      (Variables|Default|SetCurrentLife 0.0)
      (Default|CallOnDeath (Components|GetOwner))
      (if (Variables|Default|GetDestroyOnDeath)
        (Actor|DestroyActor (Components|GetOwner)))
      (else
        (Default|CallOnGetDamage (Variables|Default|GetCurrentLife) Damager)
        (Development|PrintString (Utilities|String|Append (Utilities|GetDisplayName (Components|GetOwner)) " has " (Utilities|String|ToString(Float) _output_get) " HP!"))))))