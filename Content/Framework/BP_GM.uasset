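; Game mode for a timed coin-collection level where gathering every coin opens the exit door and running out of time triggers defeat.
; On BeginPlay it restores collected coins and remaining time from the GameInstance save, counts level coins and starts a one-second countdown.
; PointsRefresh records coin IDs, updates score text and arms the door, which Tick opens.
; Victory and Defeat spawn end actors and switch music, while getters expose save data.
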(event Custom|Defeat
  ;[0 0 0] Defeat
  (Game|SpawnActorfromClass "/Game/Levels/Defeat/BP_Defeat.BP_Defeat_C" (Transformation|GetActorTransform) "Undefined" "MultiplyWithRoot" 0 0)
  (bind _outactors (Actor|GetAllActorsOfClass "/Game/SoundFX/LevelMusic.LevelMusic_C"))
  (for _array_element _outactors
    (Default|DefeatMusic _array_element)))

(event Custom|Victory
  ;[0 0 0] Victory
  (Variables|Default|SetNextLevel (Variables|/Game/Characters/BP_Door.BP_Door_C|GetNextLevel (Variables|Default|GetDoor)))
  (Game|SpawnActorfromClass "/Game/Levels/Victorory/BP_Victory.BP_Victory_C" (Transformation|GetActorTransform) "Undefined" "MultiplyWithRoot" 0 0)
  (bind _outactors (Actor|GetAllActorsOfClass "/Game/SoundFX/LevelMusic.LevelMusic_C"))
  (for _array_element _outactors
    (Default|VictoryMusic _array_element)))

(event Custom|PointsRefresh
  (params (ID :type Guid%20Structure) (Transform :type S%20Coin%20Save%20Structure))
  (bind _totalcollectibles (Variables|Default|GetTotalCollectibles))
  ;[0 0 0] Points Update
  (Utilities|Map|Add (Variables|Default|GetSessionCollectedGuids) ID Transform)
  (Development|PrintString (Guid|ToString(Guid) ID))
  (Variables|Default|SetPointsText (Utilities|String|BuildString(Integer) (Utilities|String|ToString(Integer) (- _totalcollectibles (Variables|Default|GetCollectablesLeft))) " / " _totalcollectibles))
  (if (<= (Variables|Default|GetCollectablesLeft) 0)
    (Variables|Default|SetCanOpenDoor true)))

(event Custom|OnTimerStarted
  (if (== (Variables|Default|GetSecondsRemaining) 0)
    (Variables|Default|SetSecondsRemaining 59)
    (bind _result (Math|Integer|DecrementInt (Variables|Default|GetMinutesRemaining))
      (:%20%20
        (if (== _result -1)
          (Utilities|Time|ClearandInvalidateTimerbyHandle (stale EventBeginPlay _return_value))
          (Variables|Default|SetMinutesRemaining 0)
          (Variables|Default|SetSecondsRemaining 59)
          (CallFunction|Defeat))))
    (else
      (Math|Integer|DecrementInt (Variables|Default|GetSecondsRemaining)))))

(event EventBeginPlay
  ;[0 0 0] Set References
  (bind _asbp_game_instance (Utilities|Casting|CastToBP_GameInstance (Game|GetGameInstance)))
  (Utilities|IsValid (Variables|/Game/Levels/SaveSystem/BP_GameInstance.BP_GameInstance_C|GetSaveData _asbp_game_instance)
    (:Is%20Valid
      (Variables|Default|SetSessionCollectedGuids (Variables|/Game/Levels/SaveSystem/BP_SaveGame.BP_SaveGame_C|GetCollectedCoins (Variables|/Game/Levels/SaveSystem/BP_GameInstance.BP_GameInstance_C|GetSaveData _asbp_game_instance)))
      (Variables|Default|SetInitialCollectibles (Variables|/Game/Levels/SaveSystem/BP_SaveGame.BP_SaveGame_C|GetSavedScore (Variables|/Game/Levels/SaveSystem/BP_GameInstance.BP_GameInstance_C|GetSaveData _asbp_game_instance)))
      (Variables|Default|SetMinutesRemaining (.X (Utilities|Struct|BreakIntPoint (Variables|/Game/Levels/SaveSystem/BP_SaveGame.BP_SaveGame_C|GetTimeRemaining (Variables|/Game/Levels/SaveSystem/BP_GameInstance.BP_GameInstance_C|GetSaveData _asbp_game_instance)))))
      (Variables|Default|SetSecondsRemaining (.Y (Utilities|Struct|BreakIntPoint (Variables|/Game/Levels/SaveSystem/BP_SaveGame.BP_SaveGame_C|GetTimeRemaining (Variables|/Game/Levels/SaveSystem/BP_GameInstance.BP_GameInstance_C|GetSaveData _asbp_game_instance))))))
    (:Is%20Not%20Valid
      (Development|PrintString "Failed To Load")
      (Variables|Default|SetInitialCollectibles 0)))
  (bind _outactors (Actor|GetAllActorsOfClass "/Game/Characters/BP_Coin.BP_Coin_C"))
  (bind _output_get (Variables|Default|SetCoins _outactors))
  (Variables|Default|SetCollectablesLeft (Utilities|Array|Length _output_get))
  (bind _output_get_2 (Variables|Default|SetTotalCollectibles (+ (Utilities|Array|Length _output_get) (Variables|Default|GetInitialCollectibles))))
  (Variables|Default|SetPointsText (Utilities|String|BuildString(Integer) (Utilities|String|ToString(Integer) (Variables|Default|GetInitialCollectibles)) " / " _output_get_2))
  (bind _returnvalue (Actor|GetActorOfClass "/Game/Characters/BP_Door.BP_Door_C"))
  (Variables|Default|SetDoor _returnvalue)
  (Utilities|IsValid (Variables|/Game/Levels/SaveSystem/BP_GameInstance.BP_GameInstance_C|GetSaveData _asbp_game_instance)
    (:Is%20Valid
      (if (not (Class|KismetMathLibrary|EqualIntPointIntPoint (Variables|/Game/Levels/SaveSystem/BP_SaveGame.BP_SaveGame_C|GetTimeRemaining (Variables|/Game/Levels/SaveSystem/BP_GameInstance.BP_GameInstance_C|GetSaveData _asbp_game_instance)) (Utilities|Struct|MakeIntPoint 0 0)))
        (CallFunction|StartTimer)
        (else
          (CallFunction|StartTimer))))
    (:Is%20Not%20Valid
      (bind _return_value (CallFunction|StartTimer)))))

(event EventTick
  (params (DeltaSeconds :type Float%20%28single-precision%29))
  (bind _door (Variables|Default|GetDoor))
  ;[0 0 0] Win Condition
  (if (and (<= (Variables|Default|GetCollectablesLeft) 0) (Variables|Default|GetCanOpenDoor))
    (Variables|Default|SetCanOpenDoor false)
    (Utilities|IsValid _door
      (:Is%20Valid
        (Default|OpenDoor _door))
      (:Is%20Not%20Valid
        (Development|PrintString "Puerta no Valida")))))

(fn ConstructionScript)

(fn CoinCollected
  (bind _result (Math|Integer|DecrementInt (Variables|Default|GetCollectablesLeft))
    (:%20%20
      (Variables|Default|SetCollectablesLeft _result))))

(fn StartTimer
  (bind _returnvalue (Utilities|Time|SetTimerbyEvent (EventDispatchers|CreateEvent :!event Custom|OnTimerStarted) 1.0 true))
  (return _returnvalue))

(fn GetTimerSave
  (return (Utilities|Struct|MakeIntPoint (Variables|Default|GetMinutesRemaining) (Variables|Default|GetSecondsRemaining))))

(fn GetCoinsSave
  (return (Variables|Default|GetSessionCollectedGuids)))