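; BP_EnemyCharacter is an enemy that hurts damageable actors on contact and gets knocked back when BP_Spyro damages it.
; On overlap it deals a small random, rounded amount of damage through the other actor's BPC_Damageable component, sparing Spyro while he is charging.
; Its own BPC_Damageable damage event launches it along Spyro's forward vector with added lift, scaled by Spyro's BumpForce.
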(event OnGetDamage(BPC_Damageable)
  (params (CurrentHP :type Float%20%28double-precision%29) (Damager :type Actor%20Object%20Reference))
  ;[0 0 0] Bump OnDamage
  (bind _asbp_spyro (Utilities|Casting|CastToBP_Spyro Damager))
  (Character|LaunchCharacter (Math|Vector|MakeVector (.x (+ (* (Math|Vector|GetForwardVector (Transformation|GetWorldRotation (Variables|/Script/Engine.Actor|GetRootComponent Damager))) (* (Variables|/Game/Characters/BP_Spyro.BP_Spyro_C|GetBumpForce _asbp_spyro) 3.0)) (* (Transformation|GetActorUpVector) (Variables|/Game/Characters/BP_Spyro.BP_Spyro_C|GetBumpForce _asbp_spyro)))) (.y (+ (* (Math|Vector|GetForwardVector (Transformation|GetWorldRotation (Variables|/Script/Engine.Actor|GetRootComponent Damager))) (* (Variables|/Game/Characters/BP_Spyro.BP_Spyro_C|GetBumpForce _asbp_spyro) 3.0)) (* (Transformation|GetActorUpVector) (Variables|/Game/Characters/BP_Spyro.BP_Spyro_C|GetBumpForce _asbp_spyro)))) (.z (+ (* (Math|Vector|GetForwardVector (Transformation|GetWorldRotation (Variables|/Script/Engine.Actor|GetRootComponent Damager))) (* (Variables|/Game/Characters/BP_Spyro.BP_Spyro_C|GetBumpForce _asbp_spyro) 3.0)) (* (Transformation|GetActorUpVector) (Variables|/Game/Characters/BP_Spyro.BP_Spyro_C|GetBumpForce _asbp_spyro))))) true false))

(event Collision|EventActorBeginOverlap
  (params (OtherActor :type Actor%20Object%20Reference))
  (bind _returnvalue (Actor|GetComponentbyClass OtherActor "/Game/Framework/BPC_Damageable.BPC_Damageable_C"))
  ;[0 0 0] Damage Player
  (Utilities|IsValid _returnvalue
    (:Is%20Valid
      (bind _asbp_spyro (Utilities|Casting|CastToBP_Spyro OtherActor)
        (:then
          (if (not (Variables|/Game/Characters/BP_Spyro.BP_Spyro_C|GetIsCharging? _asbp_spyro))
            (Default|GetDamage _returnvalue (Math|Conversions|ToFloat(Integer) (Math|Float|Round (Math|Random|RandomFloatinRange 5.0 1e+01))) self :!label _label)))
        (:CastFailed
          (goto _label))))))

(fn ConstructionScript)

(fn NewFunction)