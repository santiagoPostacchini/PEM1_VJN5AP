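; Double-door exit actor that triggers the game's victory once it has been opened.
; On BeginPlay it registers itself on BP_GM, exposing OpenDoor, which plays a creak sound and a timeline that swings both leaves in mirrored yaw.
; The timeline clears DoorClosed once its rotation value reaches one.
; A Box begin overlap while the door is open calls Victory on the game mode.
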(event OnComponentBeginOverlap(Box)
  (params (OverlappedComponent :type Primitive%20Component%20Object%20Reference) (OtherActor :type Actor%20Object%20Reference) (OtherComp :type Primitive%20Component%20Object%20Reference) (OtherBodyIndex :type Integer) (bFromSweep :type Boolean) (SweepResult :type Hit%20Result%20Structure%20%28by%20ref%29))
  (if (not (Variables|Default|GetDoorClosed))
    (Default|Victory (Variables|Default|GetGameMode))))

(event Custom|OpenDoor
  (if (Variables|Default|GetDoorClosed)
    (Audio|SpawnSoundatLocation "/Game/SoundFX/cue/Wood_and_Door_Creak_01_Cue.Wood_and_Door_Creak_01_Cue" (Transformation|GetActorLocation) "0, 0, 0" 1.0 1.0 0.0 0 0)
    (bind _door (Timeline|DoorRotation Play)
      (:Update
        (Transformation|SetRelativeLocationAndRotation (Variables|Default|GetDoorL) "0.000000,210.000000,0.000000" (Math|Rotator|MakeRotator 0.0 0.0 _door) false false)
        (Transformation|SetRelativeLocationAndRotation (Variables|Default|GetDoorR) "0.000000,-210.000000,0.000000" (* (Math|Rotator|MakeRotator 0.0 0.0 _door) -1.0) false false)
        (Variables|Default|SetDoorClosed (< _door 1.0))))))

(event EventBeginPlay
  (bind _returnvalue (Actor|GetActorOfClass "/Game/Framework/BP_GM.BP_GM_C"))
  (bind _output_get (Variables|Default|SetGameMode _returnvalue))
  (Variables|/Game/Framework/BP_GM.BP_GM_C|SetDoor _output_get self))

(fn ConstructionScript)