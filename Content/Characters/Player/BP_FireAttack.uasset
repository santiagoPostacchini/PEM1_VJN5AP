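; BP_FireAttack is Spyro's short-lived fire breath attack actor.
; On spawn it plays a whoosh sound and runs a Timeline, destroying itself when the Timeline finishes.
; Each tick it snaps its location and rotation to Spyro's FireSpawnTransform.
; Overlapping a BP_Mage deals heavy damage through that mage's BPCDamageable component; other actors are ignored.
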(event EventBeginPlay
  (Audio|SpawnSound2D "/Game/SoundFX/cue/Fire_Whoosh_2-15_Cue.Fire_Whoosh_2-15_Cue" 1.0 1.0 0.0 0 false false)
  (Timeline|Timeline Play
    (:Finished
      (Actor|DestroyActor))))

(event Collision|EventActorBeginOverlap
  (params (OtherActor :type Actor%20Object%20Reference))
  (bind _asbp_mage (Utilities|Casting|CastToBP_Mage OtherActor))
  (Default|GetDamage (Variables|/Game/Characters/AI/BP_Mage.BP_Mage_C|GetBPC_Damageable _asbp_mage) 1e+03 self))

(event EventTick
  (params (DeltaSeconds :type Float%20%28single-precision%29))
  (bind _spyro (Variables|Default|GetSpyro))
  (bind _firespawntransform (Variables|/Game/Characters/BP_Spyro.BP_Spyro_C|GetFireSpawnTransform _spyro))
  (Transformation|SetActorLocation (Math|Transform|TransformLocation _firespawntransform "0, 0, 0") false false)
  (Transformation|SetActorRotation (Math|Transform|TransformRotation _firespawntransform "0, 0, 0")))

(fn ConstructionScript)