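; BP_Collectable is a pickup actor that the third-person character collects by overlapping its sphere component.
; On overlap it decrements CollectablesLeft on BP_ThirdPersonGameMode and prints the collected count out of TotalCollectibles, then destroys itself.
; When the last one is collected it also prints a long-lasting Spanish "door unlocked" message, though no door logic runs here.
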(event OnComponentBeginOverlap(Sphere)
  (params (OverlappedComponent :type Primitive%20Component%20Object%20Reference) (OtherActor :type Actor%20Object%20Reference) (OtherComp :type Primitive%20Component%20Object%20Reference) (OtherBodyIndex :type Integer) (bFromSweep :type Boolean) (SweepResult :type Hit%20Result%20Structure%20%28by%20ref%29))
  (Utilities|Casting|CastToBP_ThirdPersonCharacter OtherActor)
  (bind _asbp_third_person_game_mode (Utilities|Casting|CastToBP_ThirdPersonGameMode (Game|GetGameMode)))
  (bind _result (Math|Integer|DecrementInt (Variables|/Game/ThirdPerson/Blueprints/BP_ThirdPersonGameMode.BP_ThirdPersonGameMode_C|GetCollectablesLeft _asbp_third_person_game_mode))
    (:%20%20
      (bind _output_get (Variables|/Game/ThirdPerson/Blueprints/BP_ThirdPersonGameMode.BP_ThirdPersonGameMode_C|SetCollectablesLeft _asbp_third_person_game_mode _result))
      (Development|PrintString (Utilities|String|ToString(Text) (Utilities|Text|FormatText "{X}/{Y} Colected" (- (Variables|/Game/ThirdPerson/Blueprints/BP_ThirdPersonGameMode.BP_ThirdPersonGameMode_C|GetTotalCollectibles _asbp_third_person_game_mode) _output_get) (Variables|/Game/ThirdPerson/Blueprints/BP_ThirdPersonGameMode.BP_ThirdPersonGameMode_C|GetTotalCollectibles _asbp_third_person_game_mode))))
      (if (== (- (Variables|/Game/ThirdPerson/Blueprints/BP_ThirdPersonGameMode.BP_ThirdPersonGameMode_C|GetTotalCollectibles _asbp_third_person_game_mode) _output_get) (Variables|/Game/ThirdPerson/Blueprints/BP_ThirdPersonGameMode.BP_ThirdPersonGameMode_C|GetTotalCollectibles _asbp_third_person_game_mode))
        (Development|PrintString "Puerta desbloqueada" true true "(R=0.000000,G=0.660000,B=1.000000,A=1.000000)" 2e+13))
      (Actor|DestroyActor))))

(event EventBeginPlay)

(event EventTick
  (params (DeltaSeconds :type Float%20%28single-precision%29)))

(fn ConstructionScript)