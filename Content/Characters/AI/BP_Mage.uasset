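; Mage enemy AI character that damages damageable actors on overlap, except a charging Spyro, and can spawn a trap.
; AI perception feeds Spyro into the blackboard Target.
; Hits from Spyro launch it away and disable further damage until it lands.
; A construction-time GUID keys its save of transform, health and blackboard state, restored on BeginPlay; loading a game without a matching entry destroys it.
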(event OnGetDamage(BPC_Damageable)
  (params (CurrentHP :type Float%20%28double-precision%29) (Damager :type Actor%20Object%20Reference))
  ;[0 0 0] Bump OnDamage
  (bind _asbp_spyro (Utilities|Casting|CastToBP_Spyro Damager))
  (Character|LaunchCharacter (Math|Vector|MakeVector (.x (+ (* (Math|Vector|GetForwardVector (Transformation|GetWorldRotation (Variables|/Script/Engine.Actor|GetRootComponent Damager))) (* (Variables|/Game/Characters/BP_Spyro.BP_Spyro_C|GetBumpForce _asbp_spyro) 3.0)) (* (Transformation|GetActorUpVector) (Variables|/Game/Characters/BP_Spyro.BP_Spyro_C|GetBumpForce _asbp_spyro)))) (.y (+ (* (Math|Vector|GetForwardVector (Transformation|GetWorldRotation (Variables|/Script/Engine.Actor|GetRootComponent Damager))) (* (Variables|/Game/Characters/BP_Spyro.BP_Spyro_C|GetBumpForce _asbp_spyro) 3.0)) (* (Transformation|GetActorUpVector) (Variables|/Game/Characters/BP_Spyro.BP_Spyro_C|GetBumpForce _asbp_spyro)))) (.z (+ (* (Math|Vector|GetForwardVector (Transformation|GetWorldRotation (Variables|/Script/Engine.Actor|GetRootComponent Damager))) (* (Variables|/Game/Characters/BP_Spyro.BP_Spyro_C|GetBumpForce _asbp_spyro) 3.0)) (* (Transformation|GetActorUpVector) (Variables|/Game/Characters/BP_Spyro.BP_Spyro_C|GetBumpForce _asbp_spyro))))) true false)
  (Variables|/Game/Framework/BPC_Damageable.BPC_Damageable_C|SetCanBeDamagable (Variables|Default|GetBPC_Damageable) false))

(event OnTargetPerceptionUpdated(AIPerception)
  (params (Actor :type Actor%20Object%20Reference) (Stimulus :type AI%20Stimulus%20Structure))
  (bind _asbp_spyro (Utilities|Casting|CastToBP_Spyro Actor))
  (AI|Components|Blackboard|SetValueasObject (AI|GetBlackboard (Pawn|GetController)) (Variables|AI|GetTarget) (Utilities|SelectObject _asbp_spyro 0 (.bSuccessfullySensed (Utilities|Struct|BreakAIStimulus Stimulus)))))

(event EventBeginPlay
  (bind _returnvalue (Transformation|GetActorLocation))
  (bind _returnvalue_2 (Game|GetGameInstance))
  (bind _enemyid (Variables|Default|GetEnemyID))
  (bind _returnvalue_3 (Guid|ToString(Guid) _enemyid))
  (bind (_x _y _z) (Math|Vector|BreakVector _returnvalue))
  (bind _returnvalue_4 (Utilities|String|Append "Enemy: " _returnvalue_3))
  (bind _returnvalue_5 (+ _z 1e+02))
  (bind _returnvalue_6 (Math|Vector|MakeVector _x _y _returnvalue_5))
  (bind _savegamedata (Class|BPISaveGame|GetSaveData(Message) _returnvalue_2))
  (bind _asbp_game_instance (Utilities|Casting|CastToBP_GameInstance _returnvalue_2))
  (if (.ReturnValue (Utilities|Map|Find (Variables|/Game/Levels/SaveSystem/BP_SaveGame.BP_SaveGame_C|GetEnemySaves _savegamedata) (Variables|Default|GetEnemyID)))
    (CallFunction|UseEnemySave (.Value (Utilities|Map|Find (Variables|/Game/Levels/SaveSystem/BP_SaveGame.BP_SaveGame_C|GetEnemySaves _savegamedata) (Variables|Default|GetEnemyID))))
    (Rendering|Debug|DrawDebugString _returnvalue_6 _returnvalue_4 0 "(R=0.363921,G=1.000000,B=0.047800,A=1.000000)" 9.9e+02)
    (elif (Variables|/Game/Levels/SaveSystem/BP_GameInstance.BP_GameInstance_C|GetIsLoadingGame? _asbp_game_instance)
      (Actor|DestroyActor)
      (Development|PrintString "Destroyed Enemy")
      (else
        (Rendering|Debug|DrawDebugString _returnvalue_6 _returnvalue_4 0 "(R=1.000000,G=0.000000,B=0.000000,A=1.000000)" 999.0)))))

(event Collision|EventActorBeginOverlap
  (params (OtherActor :type Actor%20Object%20Reference))
  (bind _returnvalue (Actor|GetComponentbyClass OtherActor "/Game/Framework/BPC_Damageable.BPC_Damageable_C"))
  ;[0 0 0] Damage Player
  (Utilities|FlowControl|Sequence
    (:then_0
      (Utilities|IsValid _returnvalue
        (:Is%20Valid
          (bind _asbp_spyro (Utilities|Casting|CastToBP_Spyro OtherActor)
            (:then
              (if (not (Variables|/Game/Characters/BP_Spyro.BP_Spyro_C|GetIsCharging? _asbp_spyro))
                (if (Variables|/Game/Characters/BP_Spyro.BP_Spyro_C|GetIsInvunerable? _asbp_spyro)
                  _
                  (else
                    _))
                (Default|GetDamage _returnvalue (Math|Conversions|ToFloat(Integer) (Math|Float|Round (Math|Random|RandomFloatinRange 5.0 1e+01))) self :!label _label)))
            (:CastFailed
              (goto _label))))))
    (:then_1
      (if (Actor|ActorHasTag OtherActor "dasdasd")
        (Variables|Default|SetIsGrounded true)))))

(event EventOnLanded
  (params (Hit :type Hit%20Result%20Structure%20%28by%20ref%29))
  ;[0 0 0] Bump OnDamage
  (Variables|/Game/Framework/BPC_Damageable.BPC_Damageable_C|SetCanBeDamagable (Variables|Default|GetBPC_Damageable) true))

(fn ConstructionScript
  (if (or (not (Guid|IsValidGuid (Variables|Default|GetEnemyID))) (Variables|Default|GetResetID))
    (Variables|Default|SetEnemyID (Guid|NewGuid))))

(fn SpawnTrap
  (Development|PrintString "Trap spawned")
  (Game|SpawnActorfromClass "/Game/ThirdPerson/Blueprints/TrollTrap/BP_TrollTrap2.BP_TrollTrap2_C" (Math|Conversions|ToTransform(Vector) (Transformation|GetWorldLocation (Variables|Default|GetTrapSpawn))) "Undefined" "MultiplyWithRoot" 0 0))

(fn UseEnemySave
  (params (EnemySave :type S%20Enemy%20Save%20Structure))
  (bind _returnvalue (AI|GetBlackboard 0))
  (if (not (== (.transform EnemySave) (Math|Transform|MakeTransform "0, 0, 0")))
    (Transformation|SetActorTransform (.transform EnemySave))
    (Variables|/Game/Framework/BPC_Damageable.BPC_Damageable_C|SetCurrentLife (Variables|Default|GetBPC_Damageable) (.health EnemySave))
    (Utilities|FlowControl|Sequence
      (:then_0
        (AI|Components|Blackboard|SetValueasVector _returnvalue (Variables|Default|GetDestinationKeyName) (.destination EnemySave)))
      (:then_1
        (AI|Components|Blackboard|SetValueasBool _returnvalue (Variables|Default|GetHidingKeyName) (.ishiding EnemySave)))
      (:then_2
        (AI|Components|Blackboard|SetValueasFloat _returnvalue (Variables|Default|GetLastSeenKeyName) (.lastseentime EnemySave)))
      (:then_3
        (AI|Components|Blackboard|SetValueasBool _returnvalue (Variables|Default|GetTargetKeyName) (.hastarget EnemySave))))))

(fn GetEnemySave
  (bind _returnvalue (AI|GetBlackboard 0))
  (return (Utilities|Struct|MakeS_EnemySave (Transformation|GetActorTransform) (Variables|/Game/Framework/BPC_Damageable.BPC_Damageable_C|GetCurrentLife (Variables|Default|GetBPC_Damageable)) (AI|Components|Blackboard|GetValueasVector _returnvalue (Variables|Default|GetDestinationKeyName)) (ScalableFloat|GetValueasBool _returnvalue (Variables|Default|GetHidingKeyName)) (Class|BlackboardComponent|GetValueasFloat _returnvalue (Variables|Default|GetLastSeenKeyName)) (Utilities|IsValid (AI|Components|Blackboard|GetValueasObject _returnvalue (Variables|Default|GetTargetKeyName)))) (Variables|Default|GetEnemyID)))