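; BP_Victory is an actor that runs the victory screen when play begins.
; On BeginPlay it adds the WVictory widget to the viewport, disables the player character's movement, shows the mouse cursor and calls a timed view target blend.
; A custom event enables input on the actor, whose left mouse handlers forward press and release to a WidgetInteraction component as pointer clicks.
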(event Custom|CustomEvent
  (Input|EnableInput (Game|GetPlayerController 0)))

(event EventBeginPlay
  (bind _returnvalue (Game|GetPlayerCharacter 0))
  (bind _returnvalue_2 (Game|GetPlayerController 0))
  (bind _charactermovement (Variables|/Script/Engine.Character|GetCharacterMovement _returnvalue))
  (bind _returnvalue_3 (UserInterface|CreateWidget "/Game/Levels/Victorory/WVictory.WVictory_C" (Game|GetPlayerController 0)))
  (UserInterface|Viewport|AddtoViewport _returnvalue_3 0)
  (Utilities|IsValid _charactermovement
    (:Is%20Valid
      (Pawn|Components|CharacterMovement|DisableMovement _charactermovement))
    (:Is%20Not%20Valid
      _))
  (Game|Player|SetViewTargetwithBlend _returnvalue_2 0 4.0 "VTBlend_Linear" 0.0 false)
  (Input|SetIgnoreLookInput _returnvalue_2 false)
  (Variables|/Script/Engine.PlayerController|SetbShowMouseCursor _returnvalue_2 true))

(event Input|MouseEvents|LeftMouseButton
  (params (Key :type Key%20Structure :default "None"))
  (bind _widgetinteraction1 (Variables|Default|GetWidgetInteraction1))
  (:Pressed
    (Class|WidgetInteractionComponent|PressPointerKey _widgetinteraction1 "LeftMouseButton"))
  (:Released
    (Class|WidgetInteractionComponent|ReleasePointerKey _widgetinteraction1 "LeftMouseButton")))

(fn ConstructionScript)