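; BP_SaveStatue is a save point that lets the player open the game slot selection menu.
; Overlap by BP_Spyro enables input on the statue and shows a save pop-up, while ending overlap disables input and removes both widgets.
; Pressing E sets IsLoadingGame on the game instance, creates the slot selection widget flagged as InSaveStatue, and switches to UI-only input focused on it.
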(event Collision|EventActorBeginOverlap
  (params (OtherActor :type Actor%20Object%20Reference))
  (Utilities|Casting|CastToBP_Spyro OtherActor)
  (Input|EnableInput (Game|GetPlayerController 0))
  (bind _returnvalue (UserInterface|CreateWidget "/Game/Levels/SaveSystem/W_SavePopUp.W_SavePopUp_C"))
  (UserInterface|Viewport|AddtoViewport _returnvalue 0))

(event Collision|EventActorEndOverlap
  (params (OtherActor :type Actor%20Object%20Reference))
  (bind _gameslotselection (Variables|Default|GetGameSlotSelection))
  (Input|DisableInput (Game|GetPlayerController 0))
  (Widget|RemovefromParent (stale Collision|EventActorBeginOverlap _returnvalue))
  (if (Utilities|IsValid _gameslotselection)
    (Widget|RemovefromParent _gameslotselection)))

(event Input|KeyboardEvents|E
  (params (Key :type Key%20Structure :default "None"))
  (:Pressed
    (bind _asbp_game_instance (Utilities|Casting|CastToBP_GameInstance (Game|GetGameInstance)))
    (Variables|/Game/Levels/SaveSystem/BP_GameInstance.BP_GameInstance_C|SetIsLoadingGame? _asbp_game_instance true)
    (bind _returnvalue (UserInterface|CreateWidget "/Game/Levels/Menu/WBP_GameSlotSelection.WBP_GameSlotSelection_C" 0 true))
    (bind _output_get (Variables|Default|SetGameSlotSelection _returnvalue))
    (UserInterface|Viewport|AddtoViewport _returnvalue 0)
    (Input|SetInputModeUIOnly (Game|GetPlayerController 0) _output_get "DoNotLock" false)))

(fn ConstructionScript)