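; AC_HealthComponent is an actor component that tracks an owner's current and maximum health.
; TakeDamage and Heal adjust CurrentHealth clamped between zero and MaxHealth, while ResetHealth refills it and LoadHealth sets a given value without clamping.
; Every change broadcasts OnHealthChanged with current and max values, and TakeDamage fires OnDeath whenever health is at zero, with no guard against repeat calls.
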(event EventBeginPlay)

(event EventTick
  (params (DeltaSeconds :type Float%20%28single-precision%29)))

(fn TakeDamage
  (params (Amount :type Float%20%28double-precision%29))
  (bind _output_get (Variables|Default|SetCurrentHealth (Math|Float|Clamp(Float) (- (Variables|Default|GetCurrentHealth) Amount) 0.0 (Variables|Default|GetMaxHealth))))
  (CallFunction|HealthChangedCall)
  (if (<= _output_get 0.0)
    (Default|CallOnDeath)))

(fn Heal
  (params (Amount :type Float%20%28double-precision%29))
  (Variables|Default|SetCurrentHealth (Math|Float|Clamp(Float) (+ Amount (Variables|Default|GetCurrentHealth)) 0.0 (Variables|Default|GetMaxHealth)))
  (CallFunction|HealthChangedCall))

(fn HealthChangedCall
  (Default|CallOnHealthChanged (Variables|Default|GetCurrentHealth) (Variables|Default|GetMaxHealth)))

(fn ResetHealth
  (Variables|Default|SetCurrentHealth (Variables|Default|GetMaxHealth))
  (CallFunction|HealthChangedCall))

(fn LoadHealth
  (params (NewHealth :type Float%20%28double-precision%29))
  (bind _output_get (Variables|Default|SetCurrentHealth NewHealth))
  (Default|CallOnHealthChanged _output_get (Variables|Default|GetMaxHealth)))